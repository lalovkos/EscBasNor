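; Base weapon actor that handles automatic firing, ammo and reloading, configured from a DT_Weapon row in the construction script.
; While fire is held, a gate-and-delay loop spends ammo and spawns BP_Bullet with random damage, playing weapon and character montages.
; Shots aim from the muzzle toward a trace from the aim or follow camera, plus random spread.
; Reloading refills the clip from reserve ammo, automatically on trigger release when empty.
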(event Custom|FireRelease
  (CallFunction|StopFire)
  (Variables|Default|SetCanFiing false)
  (CallFunction|AutoReload))

(event Custom|FirePress
  (CallFunction|StartFire)
  (Variables|Default|SetCanFiing true))

(event Custom|ReloadWeapon
  (if (> (.AmmoMax (Utilities|Struct|BreakStruct_WeaponData (Variables|Default|GetWeaponData))) 0)
    (Variables|Default|SetNeededAmmo (- (.AmmoInClip (Utilities|Struct|BreakStruct_WeaponData (Variables|Default|GetWeaponData))) (.AmmoCurrent (Utilities|Struct|BreakStruct_WeaponData (Variables|Default|GetWeaponData)))))
    (if (<= (Utilities|Struct|BreakStruct_WeaponData (Variables|Default|GetWeaponData)) (Variables|Default|GetNeededAmmo))
      (Variables|Default|SetWeaponData (Utilities|Struct|MakeStruct_WeaponData (.FireMode (Utilities|Struct|BreakStruct_WeaponData (Variables|Default|GetWeaponData))) (.MuzzleName (Utilities|Struct|BreakStruct_WeaponData (Variables|Default|GetWeaponData))) (.FireRate (Utilities|Struct|BreakStruct_WeaponData (Variables|Default|GetWeaponData))) (.ReloadDelay (Utilities|Struct|BreakStruct_WeaponData (Variables|Default|GetWeaponData))) (.WeaponSpread (Utilities|Struct|BreakStruct_WeaponData (Variables|Default|GetWeaponData))) (.DamageMin (Utilities|Struct|BreakStruct_WeaponData (Variables|Default|GetWeaponData))) (.DamageMax (Utilities|Struct|BreakStruct_WeaponData (Variables|Default|GetWeaponData))) 0 (.AmmoInClip (Utilities|Struct|BreakStruct_WeaponData (Variables|Default|GetWeaponData))) (+ (.AmmoCurrent (Utilities|Struct|BreakStruct_WeaponData (Variables|Default|GetWeaponData))) (.AmmoMax (Utilities|Struct|BreakStruct_WeaponData (Variables|Default|GetWeaponData))))))
      (else
        (Variables|Default|SetWeaponData (Utilities|Struct|MakeStruct_WeaponData (.FireMode (Utilities|Struct|BreakStruct_WeaponData (Variables|Default|GetWeaponData))) (.MuzzleName (Utilities|Struct|BreakStruct_WeaponData (Variables|Default|GetWeaponData))) (.FireRate (Utilities|Struct|BreakStruct_WeaponData (Variables|Default|GetWeaponData))) (.ReloadDelay (Utilities|Struct|BreakStruct_WeaponData (Variables|Default|GetWeaponData))) (.WeaponSpread (Utilities|Struct|BreakStruct_WeaponData (Variables|Default|GetWeaponData))) (.DamageMin (Utilities|Struct|BreakStruct_WeaponData (Variables|Default|GetWeaponData))) (.DamageMax (Utilities|Struct|BreakStruct_WeaponData (Variables|Default|GetWeaponData))) (- (.AmmoMax (Utilities|Struct|BreakStruct_WeaponData (Variables|Default|GetWeaponData))) (Variables|Default|GetNeededAmmo)) (.AmmoInClip (Utilities|Struct|BreakStruct_WeaponData (Variables|Default|GetWeaponData))) (.AmmoInClip (Utilities|Struct|BreakStruct_WeaponData (Variables|Default|GetWeaponData)))))))))

(event Custom|StartFire
  (if (not (Variables|Default|GetIsReloading))
    (switch Utilities|FlowControl|Switch|SwitchonEnum_FireMode (Variables|Default|GetFire%20Mode)
      (:NewEnumerator2
        (Utilities|FlowControl|Sequence
          (:then_0
            (goto _label Open))
          (:then_1
            (Utilities|FlowControl|Gate true :!label _label
              (:Exit
                (Utilities|FlowControl|Sequence
                  (:then_0
                    (Utilities|FlowControl|Delay (Variables|Default|GetFire%20Rate))
                    (goto _label))
                  (:then_1
                    (if (> (Utilities|Struct|BreakStruct_WeaponData (Variables|Default|GetWeaponData)) 0)
                      (CallFunction|SpawnProjectile)
                      (Variables|Default|SetWeaponData (Utilities|Struct|MakeStruct_WeaponData (.FireMode (Utilities|Struct|BreakStruct_WeaponData (Variables|Default|GetWeaponData))) (.MuzzleName (Utilities|Struct|BreakStruct_WeaponData (Variables|Default|GetWeaponData))) (.FireRate (Utilities|Struct|BreakStruct_WeaponData (Variables|Default|GetWeaponData))) (.ReloadDelay (Utilities|Struct|BreakStruct_WeaponData (Variables|Default|GetWeaponData))) (.WeaponSpread (Utilities|Struct|BreakStruct_WeaponData (Variables|Default|GetWeaponData))) (.DamageMin (Utilities|Struct|BreakStruct_WeaponData (Variables|Default|GetWeaponData))) (.DamageMax (Utilities|Struct|BreakStruct_WeaponData (Variables|Default|GetWeaponData))) (.AmmoMax (Utilities|Struct|BreakStruct_WeaponData (Variables|Default|GetWeaponData))) (.AmmoInClip (Utilities|Struct|BreakStruct_WeaponData (Variables|Default|GetWeaponData))) (- (.AmmoCurrent (Utilities|Struct|BreakStruct_WeaponData (Variables|Default|GetWeaponData))) 1) (.FiringMontage (Utilities|Struct|BreakStruct_WeaponData (Variables|Default|GetWeaponData))) (.ReloadMontage (Utilities|Struct|BreakStruct_WeaponData (Variables|Default|GetWeaponData))))))))))))))))

(event Custom|StopFire
  (Utilities|FlowControl|Gate true) ; enters at Close
)

(event Custom|AutoReload
  (bind _weapondata (Variables|Default|GetWeaponData))
  (bind (_ammomax _ammocurrent) (Utilities|Struct|BreakStruct_WeaponData _weapondata))
  (if (== _ammocurrent 0)
    (if (not (== _ammomax 0))
      (Variables|Default|SetIsReloading true)
      (CallFunction|Reloading)
      (Utilities|FlowControl|Delay (Utilities|Struct|BreakStruct_WeaponData (Variables|Default|GetWeaponData)))
      (Variables|Default|SetIsReloading false))))

(event Custom|Reloading
  (bind _weapondata (Variables|Default|GetWeaponData))
  (bind (_ammomax _ammoinclip _ammocurrent) (Utilities|Struct|BreakStruct_WeaponData _weapondata))
  (if (not (Variables|Default|GetCanFiing))
    (if (not (== _ammomax 0))
      (if (not (== _ammoinclip _ammocurrent))
        (bind _output_get (Variables|Default|SetIsReloading true))
        (if _output_get
          (CallFunction|ReloadWeapon)
          (CallFunction|PlayMontage (Utilities|Struct|BreakStruct_WeaponData (Variables|Default|GetWeaponData)) "/Game/Anim/AnimStarterPack/Montage/Reload_Rifle_Hip_Montage.Reload_Rifle_Hip_Montage")
          (Utilities|FlowControl|Delay (Utilities|Struct|BreakStruct_WeaponData (Variables|Default|GetWeaponData)))
          (Variables|Default|SetIsReloading false))))))

(fn ConstructionScript
  (bind _returnvalue (Utilities|GetDataTableRow "/Game/Blueprints/Weapon/DT_Weapon.DT_Weapon" (Variables|Default|GetWeaponRowName))
    (:then
      (bind _output_get (Variables|Default|SetWeaponData _returnvalue))
      (Variables|Default|SetFire%20Mode (.FireMode (Utilities|Struct|BreakStruct_WeaponData _output_get)))
      (Variables|Default|SetMuzzle%20Name (.MuzzleName (Utilities|Struct|BreakStruct_WeaponData _output_get)))
      (Variables|Default|SetFire%20Rate (.FireRate (Utilities|Struct|BreakStruct_WeaponData _output_get)))
      (Variables|Default|SetReload%20Delay (.ReloadDelay (Utilities|Struct|BreakStruct_WeaponData _output_get)))
      (Variables|Default|SetWeapon%20Spread (.WeaponSpread (Utilities|Struct|BreakStruct_WeaponData _output_get))))))

(fn CalculateDirection
  (bind _returnvalue (Utilities|MuzzlePosition))
  (bind _charref (Variables|Default|GetCharRef))
  (bind _weaponcamera (Variables|Default|GetWeaponCamera))
  (bind _fcamera (Variables|/Game/Blueprints/BP_PlayerCharacter.BP_PlayerCharacter_C|GetFCamera _charref))
  (bind _aiming (Variables|/Game/Blueprints/BP_PlayerCharacter.BP_PlayerCharacter_C|GetAiming _charref))
  (bind _returnvalue_2 (select _aiming _weaponcamera _fcamera))
  (bind _returnvalue_3 (Transformation|GetWorldTransform _returnvalue_2))
  (bind _end (|EndPoint (.location _returnvalue_3) (.rotation _returnvalue_3)))
  (bind (_outhit _returnvalue_4) (Collision|LineTraceForObjects (|StartPoint (.location _returnvalue_3) (.rotation _returnvalue_3)) _end (Utilities|Array|MakeArray "ObjectTypeQuery1") false 0 "None"))
  (return _returnvalue (Math|Rotator|FindLookatRotation _returnvalue (Math|Vector|SelectVector (.ImpactPoint (Collision|BreakHitResult _outhit)) _end _returnvalue_4))))

(fn SpawnProjectile
  (bind _weapondata (Variables|Default|GetWeaponData))
  (bind (_damagemin _damagemax) (Utilities|Struct|BreakStruct_WeaponData _weapondata))
  (CallFunction|PlayMontage (Utilities|Struct|BreakStruct_WeaponData (Variables|Default|GetWeaponData)) (select (Variables|/Game/Blueprints/BP_PlayerCharacter.BP_PlayerCharacter_C|GetAiming (Variables|Default|GetCharRef)) "/Game/Anim/AnimStarterPack/Montage/Fire_Rifle_Ironsights_Montage.Fire_Rifle_Ironsights_Montage" "/Game/Anim/AnimStarterPack/Montage/Fire_Rifle_Hip_Montage.Fire_Rifle_Hip_Montage"))
  (bind (_location _rotation) (CallFunction|CalculateDirection))
  (bind _transform (CallFunction|CalculateFinalDirection _location _rotation))
  (Game|SpawnActorfromClass "/Game/Blueprints/Weapon/BP_Bullet.BP_Bullet_C" _transform "Undefined" 0 (Math|Random|RandomFloatinRange _damagemin _damagemax) 0))

(fn CalculateFinalDirection
  (params (Location :type Vector) (Rotation :type Rotator))
  (bind _weapon_spread (Variables|Default|GetWeapon%20Spread))
  (bind _returnvalue (* _weapon_spread -1.0))
  (return (Math|Transform|MakeTransform Location (Math|Rotator|CombineRotators Rotation (Math|Rotator|MakeRotator (Math|Random|RandomFloatinRange _returnvalue 0.0) (Math|Random|RandomFloatinRange _returnvalue 0.0) (Math|Random|RandomFloatinRange _returnvalue 0.0))))))

(fn PlayMontage
  (params (WeaponAnim :type Anim%20Montage%20Object%20Reference) (CharAnim :type Anim%20Montage%20Object%20Reference))
  (Animation|Montage|MontagePlay (Components|SkeletalMesh|GetAnimInstance (Variables|Default|GetWeaponMesh)) WeaponAnim 1.0 "MontageLength" 0.0 true)
  (Animation|Montage|MontagePlay (Components|SkeletalMesh|GetAnimInstance (Variables|/Script/Engine.Character|GetMesh (Variables|Default|GetCharRef))) CharAnim 1.0 "MontageLength" 0.0 true))